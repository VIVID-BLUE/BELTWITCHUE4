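; Trigger-box spawner that releases a wave of BP_MannequinFighter_AI enemies the first time the player character overlaps it.
; After caching the combat game mode, it loops with a delay, taking each spawn's wait and location from SpawnEnemy.
; Each enemy is registered with the game mode's enemy list and its first AI manager.
; The spawner destroys itself once the count reaches MaxEnemies.
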(event OnComponentBeginOverlap(Box)
  (params (OverlappedComponent :type Primitive%20Component%20Object%20Reference) (OtherActor :type Actor%20Object%20Reference) (OtherComp :type Primitive%20Component%20Object%20Reference) (OtherBodyIndex :type Integer) (bFromSweep :type Boolean) (SweepResult :type Hit%20Result%20Structure%20%28by%20ref%29))
  (if (== OtherActor (Game|GetPlayerCharacter 0))
    (if (not (Variables|Default|GetIsActive))
      (Variables|Default|SetIsActive true)
      (bind _asgm_combat_game_mode (Utilities|Casting|CastToGM_CombatGameMode (Game|GetGameMode)))
      (Variables|Default|SetGameModeRef _asgm_combat_game_mode)
      (bind (_speed _offset) (Class|AISpawnerBase|SpawnEnemy :!label _label))
      (Utilities|FlowControl|Delay _speed)
      (bind _returnvalue (Game|SpawnActorfromClass "/Game/StylishCombatKit/Characters/BP_MannequinFighter_AI.BP_MannequinFighter_AI_C" (Math|Conversions|ToTransform(Vector) _offset) "AdjustIfPossibleButAlwaysSpawn" 0 0))
      (CallFunction|AddEnemytoArray _returnvalue)
      (Math|Integer|IncrementInt (Variables|Default|GetEnemyCount)
        (:%20%20
          (if (< (Variables|Default|GetEnemyCount) (Variables|Default|GetMaxEnemies))
            (goto _label)
            (else
              (Actor|DestroyActor))))))))

(event Collision|EventActorBeginOverlap
  (params (OtherActor :type Actor%20Object%20Reference)))

(fn ConstructionScript)

(fn AddEnemytoArray
  (params (InputPin :type BP%20Mannequin%20Fighter%20AI%20Object%20Reference))
  (bind _gamemoderef (Variables|Default|GetGameModeRef))
  (Utilities|Array|Add (Variables|/Game/StylishCombatKit/AI/BP_AI_Manager.BP_AI_Manager_C|GetAI_Characters (Utilities|Array|Get(acopy) (Variables|/Game/StylishCombatKit/Main/GM_CombatGameMode.GM_CombatGameMode_C|GetAIManagers _gamemoderef))) InputPin)
  (Utilities|Array|Add (Variables|/Game/StylishCombatKit/Main/GM_CombatGameMode.GM_CombatGameMode_C|GetEnemies _gamemoderef) InputPin))