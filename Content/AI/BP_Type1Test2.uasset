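; Test AI fighter character (Type 1) that locks on to the player and plays hit reactions.
; On BeginPlay it runs the parent setup, then sets the player's BP_BaseCharacter as its lock-on target.
; HurtAnimation picks an air, long or standard hitstun montage based on airborne state and whether the struck capsule is a weak hurtbox.
; It then updates action permissions, disables enemy step and changes the state index.
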(event EventBeginPlay
  ;[1 1 1] Initialize
  (|CallParentFunction)
  (bind _asbp_base_character (Utilities|Casting|CastToBP_BaseCharacter (Game|GetPlayerCharacter 0)))
  (Variables|Default|SetLockOnTarget _asbp_base_character)
  (Variables|Default|SetIsLockedOn true)
  (Variables|Default|SetLockonButton true))

(event Collision|EventActorBeginOverlap
  (params (OtherActor :type Actor%20Object%20Reference)))

(event EventTick
  (params (DeltaSeconds :type Float%20%28single-precision%29))
  (|CallParentFunction DeltaSeconds) ; This node is disabled and will not be called.\nDrag off pins to build functionality.
)

(event EventHurtAnimation
  (params (AttackerHitbox :type BP%20Hitbox%20Object%20Reference) (HitData :type Struct%20Hit%20Data%20Structure) (HitResult :type Hit%20Result%20Structure))
  ;[1 0.09166 0.6459] Hit Event
  (if (Variables|Default|GetInAir)
    (Animation|PlayAnimMontage "/Game/StylishCombatKit/Characters/FighterAnimations/Hurt/Fighter_Hitstun_air_Montage.Fighter_Hitstun_air_Montage" 1.0 "")
    (else
      (bind _ascapsule_collision (Utilities|Casting|CastToCapsuleComponent (.HitComponent (Collision|BreakHitResult HitResult)))
        (:then
          (Animation|PlayAnimMontage (select (Utilities|Array|ContainsItem (Variables|Default|GetWeakHurtboxes) _ascapsule_collision) "/Game/StylishCombatKit/Characters/FighterAnimations/Hurt/Fighter_Hitstun_long_Montage.Fighter_Hitstun_long_Montage" "/Game/StylishCombatKit/Characters/FighterAnimations/Hurt/Fighter_Hitstun_Montage.Fighter_Hitstun_Montage") 1.0 ""))
        (:CastFailed
          (Animation|PlayAnimMontage "/Game/StylishCombatKit/Characters/FighterAnimations/Hurt/Fighter_Hitstun_Montage.Fighter_Hitstun_Montage" 1.0 "")))))
  (CallFunction|StartAnim)
  (CallFunction|CanDo false true)
  (Variables|Default|SetCanEnemyStep false)
  (Variables|Default|SetStateIndex 4))

(fn ConstructionScript
  (|CallParentFunction))