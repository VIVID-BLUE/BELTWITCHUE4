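; Manager actor that tracks target dummy AI characters and registers itself with the combat game mode.
; On BeginPlay it fills AIDummyCharacters with the first BP_Type1Test2 found plus every BP_TargetDummy, with an extra unset element appended to the latter list before copying.
; It then caches GM_CombatGameMode and adds itself to that mode's AIManagers array.
; It has no active tick or overlap logic.
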(event Collision|EventActorBeginOverlap
  (params (OtherActor :type Actor%20Object%20Reference)))

(event EventTick
  (params (DeltaSeconds :type Float%20%28single-precision%29)))

(event EventBeginPlay
  (Utilities|FlowControl|Sequence
    (:then_0
      ;[1 1 1] Populate Dummy array
      (bind _returnvalue (Actor|GetActorOfClass "/Game/AI/BP_Type1Test2.BP_Type1Test2_C"))
      (Utilities|Array|Add (Variables|Default|GetAIDummyCharacters) _returnvalue)
      (bind _outactors (Actor|GetAllActorsOfClass "/Game/AI/BP_TargetDummy.BP_TargetDummy_C"))
      (Utilities|Array|Add _outactors 0)
      (for _array_element _outactors
        (Utilities|Array|Add (Variables|Default|GetAIDummyCharacters) _array_element)))
    (:then_1
      (bind _asgm_combat_game_mode (Utilities|Casting|CastToGM_CombatGameMode (Game|GetGameMode)))
      (bind _output_get (Variables|Default|SetGameModeRef _asgm_combat_game_mode))
      (Utilities|Array|Add (Variables|/Game/StylishCombatKit/Main/GM_CombatGameMode.GM_CombatGameMode_C|GetAIManagers _output_get) self))))

(fn ConstructionScript
  (|CallParentFunction))