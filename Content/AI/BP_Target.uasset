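; BP_Target is a player-triggered overlap actor that returns its associated target dummy to its start location.
; Player begin-overlap fires a DoOnce gate, which re-arms one second after the player leaves.
; The gate looks up the dummy by EnemyIndexPosition in the BP_TargetDummyManager held in GM_CombatGameMode's AIManagers array, then moves it to its stored StartLocation.
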(event EventBeginPlay)

(event Collision|EventActorBeginOverlap
  (params (OtherActor :type Actor%20Object%20Reference))
  (if (== OtherActor (Game|GetPlayerCharacter 0))
    (Utilities|FlowControl|DoOnce false
      (:Completed
        (bind _asgm_combat_game_mode (Utilities|Casting|CastToGM_CombatGameMode (Game|GetGameMode)))
        (bind _output_get (CallFunction|GetDummyReference (Utilities|Array|Get(acopy) (Variables|/Game/StylishCombatKit/Main/GM_CombatGameMode.GM_CombatGameMode_C|GetAIManagers _asgm_combat_game_mode) 1)))
        (CallFunction|ResetDummyLocation _output_get)))))

(event EventTick
  (params (DeltaSeconds :type Float%20%28single-precision%29)))

(event Collision|EventActorEndOverlap
  (params (OtherActor :type Actor%20Object%20Reference))
  (if (== OtherActor (Game|GetPlayerCharacter 0))
    (Utilities|FlowControl|Delay 1.0)
    (Utilities|FlowControl|DoOnce false) ; enters at Reset
  ))

(fn ConstructionScript)

(fn ResetDummyLocation
  (params (Object :type Object%20Object%20Reference))
  (bind _asbp_target_dummy (Utilities|Casting|CastToBP_TargetDummy Object))
  (Transformation|SetActorLocation _asbp_target_dummy (Variables|/Game/AI/BP_TargetDummy.BP_TargetDummy_C|GetStartLocation _asbp_target_dummy) false false))

(fn GetDummyReference
  (params (Object :type Object%20Object%20Reference))
  (bind _asbp_target_dummy_manager (Utilities|Casting|CastToBP_TargetDummyManager Object))
  (bind _output_get (Variables|Default|SetDummyRef (Utilities|Array|Get(acopy) (Variables|/Game/AI/BP_TargetDummyManager.BP_TargetDummyManager_C|GetAIDummyCharacters _asbp_target_dummy_manager) (Variables|Default|GetEnemyIndexPosition))))
  (return _output_get))