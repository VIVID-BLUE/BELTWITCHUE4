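; BP_TargetSwitch is an overlap-triggered switch that toggles a target dummy's movement when the player steps on it.
; Deactivating finds the dummy by index through the game mode's target dummy manager, disables its movement and returns it to its Blackboard StartLocation.
; Activating restores walking on that cached dummy reference.
; A DoOnce gates the toggle and re-arms one second after the player leaves.
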(event EventBeginPlay)

(event Collision|EventActorBeginOverlap
  (params (OtherActor :type Actor%20Object%20Reference))
  (bind _returnvalue (Game|GetPlayerCharacter 0))
  (bind _returnvalue_2 (== OtherActor _returnvalue))
  (if _returnvalue_2
    (Utilities|FlowControl|DoOnce false
      (:Completed
        (if (Variables|Default|GetIsActive)
          (if _returnvalue_2
            (bind _asgm_combat_game_mode (Utilities|Casting|CastToGM_CombatGameMode (Game|GetGameMode)))
            (bind _output_get (CallFunction|GetDummyReference (Utilities|Array|Get(acopy) (Variables|/Game/StylishCombatKit/Main/GM_CombatGameMode.GM_CombatGameMode_C|GetAIManagers _asgm_combat_game_mode) 1)))
            (CallFunction|DisableMovementandResetLocation _output_get)
            (Variables|Default|SetIsActive false))
          (else
            (CallFunction|EnableDummyMovement)))))))

(event EventTick
  (params (DeltaSeconds :type Float%20%28single-precision%29)))

(event Collision|EventActorEndOverlap
  (params (OtherActor :type Actor%20Object%20Reference))
  (if (== OtherActor (Game|GetPlayerCharacter 0))
    (Utilities|FlowControl|Delay 1.0)
    (Utilities|FlowControl|DoOnce false) ; enters at Reset
  ))

(fn ConstructionScript)

(fn EnableDummyMovement
  (bind _asbp_type_1test_2 (Utilities|Casting|CastToBP_Type1Test2 (Variables|Default|GetDummyRef)))
  (Pawn|Components|CharacterMovement|SetMovementMode (Variables|/Script/Engine.Character|GetCharacterMovement _asbp_type_1test_2) "MOVE_Walking" 0)
  (Variables|Default|SetIsActive true))

(fn DisableMovementandResetLocation
  (params (Object :type Object%20Object%20Reference))
  (bind _asbp_type_1test_2 (Utilities|Casting|CastToBP_Type1Test2 Object))
  (Pawn|Components|CharacterMovement|DisableMovement (Variables|/Script/Engine.Character|GetCharacterMovement _asbp_type_1test_2))
  (Transformation|SetActorLocation _asbp_type_1test_2 (AI|Components|Blackboard|GetValueasVector (AI|GetBlackboard _asbp_type_1test_2) (Utilities|Name|MakeLiteralName "StartLocation")) false false))

(fn GetDummyReference
  (params (Object :type Object%20Object%20Reference))
  (bind _asbp_target_dummy_manager (Utilities|Casting|CastToBP_TargetDummyManager Object))
  (bind _output_get (Variables|Default|SetDummyRef (Utilities|Array|Get(acopy) (Variables|/Game/AI/BP_TargetDummyManager.BP_TargetDummyManager_C|GetAIDummyCharacters _asbp_target_dummy_manager) (Variables|Default|GetEnemyIndexPosition))))
  (return _output_get))