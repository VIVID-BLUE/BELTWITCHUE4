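; Standalone player camera actor for a combat game that registers with the game mode and becomes the view target.
; Each tick it interpolates location, rotation, spring-arm length and FOV, framing player and target on lock-on, otherwise following over the shoulder.
; With TrackReticle on, unlocked rotation follows reticle overshoot, and screen-side detection of character and reticle drives shoulder swaps.
; Manual rotation pauses during resets toward movement input or player facing.
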(event Custom|SetLocation
  (bind _returnvalue (Transformation|GetActorRotation))
  (bind _playerref (Variables|Default|GetPlayerRef))
  (bind _playerref_2 (Variables|Default|GetPlayerRef))
  (bind _playerref_3 (Variables|Default|GetPlayerRef))
  (bind _camera (Variables|Default|GetCamera))
  (bind _playerref_4 (Variables|Default|GetPlayerRef))
  (bind _camera_2 (Variables|Default|GetCamera))
  (bind _returnvalue_2 (Transformation|GetActorLocation _playerref_3))
  (bind _returnvalue_3 (Transformation|GetWorldLocation _camera_2))
  (bind _returnvalue_4 (Transformation|GetWorldRotation _camera_2))
  (bind _returnvalue_5 (Transformation|GetWorldRotation _camera))
  (bind _lockontarget (Variables|/Game/StylishCombatKit/Main/BP_BaseCharacter.BP_BaseCharacter_C|GetLockOnTarget _playerref_3))
  (bind _reticleref (Variables|/Game/StylishCombatKit/Main/BP_BaseCharacter.BP_BaseCharacter_C|GetReticleRef _playerref))
  (bind _reticleref_2 (Variables|/Game/StylishCombatKit/Main/BP_BaseCharacter.BP_BaseCharacter_C|GetReticleRef _playerref_4))
  (bind _returnvalue_6 (Transformation|GetActorLocation _reticleref_2))
  (bind _returnvalue_7 (Transformation|GetActorLocation _lockontarget))
  (bind _maxyaw (Variables|/Game/Blueprints/BP_Reticle.BP_Reticle_C|GetMaxYaw _reticleref))
  (bind _maxpitch (Variables|/Game/Blueprints/BP_Reticle.BP_Reticle_C|GetMaxPitch _reticleref))
  (bind _returnvalue_8 (- _returnvalue_6 _returnvalue_3))
  (bind _returnvalue_9 (* _maxyaw -1.0))
  (bind _returnvalue_10 (* _maxpitch -1.0))
  (bind _returnvalue_11 (Math|Vector|UnrotateVector _returnvalue_8 _returnvalue_4))
  (bind _returnvalue_12 (Math|Rotator|MakeRotfromX _returnvalue_11))
  (bind (_roll _pitch _yaw) (Math|Rotator|BreakRotator _returnvalue_12))
  (bind _returnvalue_13 (Math|Rotator|MakeRotator 0.0 _pitch _yaw))
  (bind (_roll_2 _pitch_2 _yaw_2) (Math|Rotator|BreakRotator _returnvalue_13))
  (bind _returnvalue_14 (Math|Float|Clamp(Float) _yaw_2 _returnvalue_9 _maxyaw))
  (bind _returnvalue_15 (Math|Float|Clamp(Float) _pitch_2 _returnvalue_10 _maxpitch))
  (bind _returnvalue_16 (Math|Rotator|MakeRotator 0.0 _returnvalue_15 _returnvalue_14))
  (bind _returnvalue_17 (Math|Rotator|Delta(Rotator) _returnvalue_13 _returnvalue_16))
  (bind _returnvalue_18 (Math|Rotator|CombineRotators _returnvalue_17 _returnvalue))
  (bind (_roll_3 _pitch_3 _yaw_3) (Math|Rotator|BreakRotator _returnvalue_18))
  ;[1 1 1] Update camera location
  (Utilities|IsValid _playerref_2
    (:Is%20Valid
      (if (Variables|/Game/StylishCombatKit/Main/BP_BaseCharacter.BP_BaseCharacter_C|GetIsLockedOn _playerref_2)
        (Transformation|SetActorLocation (Math|Interpolation|VInterpTo (Transformation|GetActorLocation) (Math|Vector|Lerp(Vector) _returnvalue_2 _returnvalue_7 (Math|Float|MapRangeClamped (- (.X (Math|Vector|BreakVector (Math|Vector|UnrotateVector _returnvalue_2 _returnvalue_5))) (.X (Math|Vector|BreakVector (Math|Vector|UnrotateVector _returnvalue_7 _returnvalue_5)))) -5e+03 5e+03 0.0 1.0)) (Utilities|Time|GetWorldDeltaSeconds) (* (Variables|Default|GetLockOnInterpSpeed) 3.0)) false false)
        (else
          (Transformation|SetActorLocation (Math|Interpolation|VInterpTo (Transformation|GetActorLocation) (+ (Transformation|GetActorLocation (Variables|Default|GetPlayerRef)) (* (Transformation|GetActorRightVector) (* (Variables|Default|GetCamSide) 1e+02)) "0,0,50.000000") (Utilities|Time|GetWorldDeltaSeconds) (* (Variables|Default|GetUnlockInterpSpeed) 1.5)) false false)
          (if (Variables|Default|GetTrackReticle)
            (Transformation|SetActorRotation (Math|Rotator|MakeRotator 0.0 (Math|Float|Clamp(Float) _pitch_3 -85.0 85.0) _yaw_3))
            (CallFunction|CamUpdateReticle)))))))

(event Custom|SetRotation
  (bind _returnvalue (Transformation|GetActorRotation))
  (bind _returnvalue_2 (Transformation|GetActorRotation))
  (bind _charside (Variables|Default|GetCharSide))
  (bind _playerref (Variables|Default|GetPlayerRef))
  (bind _returnvalue_3 (Transformation|GetActorLocation _playerref))
  (bind (_roll _pitch _yaw) (Math|Rotator|BreakRotator _returnvalue))
  (bind _lockontarget (Variables|/Game/StylishCombatKit/Main/BP_BaseCharacter.BP_BaseCharacter_C|GetLockOnTarget _playerref))
  (bind _returnvalue_4 (Transformation|GetActorLocation _lockontarget))
  (bind _returnvalue_5 (Transformation|GetHorizontalDistanceTo _playerref _lockontarget))
  (bind _returnvalue_6 (Math|Rotator|FindLookatRotation _returnvalue_3 _returnvalue_4))
  (bind _returnvalue_7 (Math|Float|MapRangeClamped _returnvalue_5 0.0 1e+02 179.0 2e+01))
  (bind _yaw_2 (Math|Rotator|BreakRotator _returnvalue_6))
  (bind _returnvalue_8 (Math|Rotator|MakeRotator 0.0 0.0 _yaw_2))
  ;[1 1 1] Update camera rotation
  (if (Variables|/Game/StylishCombatKit/Main/BP_BaseCharacter.BP_BaseCharacter_C|GetIsLockedOn (Variables|Default|GetPlayerRef))
    (Variables|Default|SetResetting false)
    (Transformation|SetActorRotation (Math|Interpolation|RInterpTo _returnvalue_2 (Math|Rotator|MakeRotator 0.0 -1e+01 (Math|Float|ClampAngle (.Yaw (Math|Rotator|BreakRotator _returnvalue_2)) (.Yaw (Math|Rotator|BreakRotator (Math|Rotator|CombineRotators _returnvalue_8 (Math|Rotator|MakeRotator 0.0 0.0 (* _returnvalue_7 -1.0))))) (.Yaw (Math|Rotator|BreakRotator (Math|Rotator|CombineRotators _returnvalue_8 (Math|Rotator|MakeRotator 0.0 0.0 _returnvalue_7)))))) (Utilities|Time|GetWorldDeltaSeconds) (Variables|Default|GetLockOnInterpSpeed)))
    (if (<= (Math|Float|Absolute(Float) (- (Variables|Default|GetCharSide) (Variables|Default|GetReticleSide))) 0.01)
      (Transformation|AddActorLocalRotation (Math|Rotator|MakeRotator 0.0 0.0 (* (select (== _charside 0.0) 1.0 (Math|Float|Sign(Float) _charside)) (- 1.0 (* (Math|Float|Absolute(Float) _charside) 1e+02)) 1.0)) false false))
    (else
      (Transformation|SetActorRotation (Math|Interpolation|RInterpTo _returnvalue (Math|Rotator|SelectRotator (Variables|Default|GetResetRotation) (Math|Rotator|MakeRotator 0.0 (Math|Float|Clamp(Float) _pitch -6e+01 6e+01) _yaw) (Variables|Default|GetResetting)) (Utilities|Time|GetWorldDeltaSeconds) (* (Variables|Default|GetUnlockInterpSpeed) 1.5)))
      (if (Math|Rotator|Equal(Rotator) (Variables|Default|GetResetRotation) (Transformation|GetActorRotation) 5.0)
        (Variables|Default|SetResetting false)
        (elif (Variables|Default|GetResetting)
          (Variables|/Game/Blueprints/BP_Reticle.BP_Reticle_C|SetAngleOffset (Variables|/Game/StylishCombatKit/Main/BP_BaseCharacter.BP_BaseCharacter_C|GetReticleRef (Variables|Default|GetPlayerRef)) "5.000000, 0, 0"))))))

(event Custom|SetZoom
  (bind _playerref (Variables|Default|GetPlayerRef))
  (bind _returnvalue (Transformation|GetActorLocation _playerref))
  ;[1 1 1] Update camera zoom
  (if (Variables|/Game/StylishCombatKit/Main/BP_BaseCharacter.BP_BaseCharacter_C|GetIsLockedOn (Variables|Default|GetPlayerRef))
    (Variables|/Script/Engine.SpringArmComponent|SetTargetArmLength (Variables|Default|GetSpringArm) (Math|Interpolation|FInterpTo (Variables|/Script/Engine.SpringArmComponent|GetTargetArmLength (Variables|Default|GetSpringArm)) (+ (* (Math|Vector|VectorLength (* (- (Transformation|GetActorLocation (Variables|/Game/StylishCombatKit/Main/BP_BaseCharacter.BP_BaseCharacter_C|GetLockOnTarget _playerref)) _returnvalue) "0.500000,0.500000,1.000000")) (Math|Float|MapRangeClamped (Math|Float|Absolute(Float) (Math|Vector|DotProduct "1.000000, 0, 0" (Math|Vector|Normalize (* (Math|Vector|UnrotateVector (Math|Vector|GetUnitDirection(Vector) (Transformation|GetActorLocation) _returnvalue) (Transformation|GetActorRotation)) "1.000000,1.000000,2.000000")))) 0.0 1.0 1.0 0.5)) (Variables|Default|GetLockonArmLengthOffset)) (Utilities|Time|GetWorldDeltaSeconds) (* (Variables|Default|GetLockOnInterpSpeed) 2.5)))
    (else
      (Variables|/Script/Engine.SpringArmComponent|SetTargetArmLength (Variables|Default|GetSpringArm) (Math|Interpolation|FInterpTo (Variables|/Script/Engine.SpringArmComponent|GetTargetArmLength (Variables|Default|GetSpringArm)) (Variables|Default|GetDefaultArmLength) (Utilities|Time|GetWorldDeltaSeconds) (* (Variables|Default|GetUnlockInterpSpeed) 1.5))))))

(event Custom|SetFOV
  (bind _playerref (Variables|Default|GetPlayerRef))
  (bind _camera (Variables|Default|GetCamera))
  (Camera|SetFieldOfView _camera (Math|Interpolation|FInterpTo (Variables|/Script/Engine.CameraComponent|GetFieldOfView _camera) (select (and (Variables|/Game/StylishCombatKit/Main/BP_BaseCharacter.BP_BaseCharacter_C|GetFocusAim _playerref) (not (Variables|/Game/StylishCombatKit/Main/BP_BaseCharacter.BP_BaseCharacter_C|GetIsLockedOn _playerref))) 7e+01 1e+02) (Utilities|Time|GetWorldDeltaSeconds) 1e+01)))

(event Custom|DetectSide
  (bind _playerref (Variables|Default|GetPlayerRef))
  (bind _camera (Variables|Default|GetCamera))
  (bind _camera_2 (Variables|Default|GetCamera))
  (bind _playerref_2 (Variables|Default|GetPlayerRef))
  (bind _playerref_3 (Variables|Default|GetPlayerRef))
  (bind _returnvalue (Transformation|GetWorldLocation _camera))
  (bind _returnvalue_2 (Transformation|GetActorLocation _playerref))
  (bind _returnvalue_3 (Transformation|GetWorldLocation _camera_2))
  (bind _reticleref (Variables|/Game/StylishCombatKit/Main/BP_BaseCharacter.BP_BaseCharacter_C|GetReticleRef _playerref_2))
  (bind _islockedon (Variables|/Game/StylishCombatKit/Main/BP_BaseCharacter.BP_BaseCharacter_C|GetIsLockedOn _playerref_3))
  (bind _returnvalue_4 (- _returnvalue_2 _returnvalue))
  (bind _returnvalue_5 (Transformation|GetActorLocation _reticleref))
  (bind _returnvalue_6 (select _islockedon 0.004 0.02))
  (bind _returnvalue_7 (- _returnvalue_5 _returnvalue_3))
  (bind _output_get (Variables|Default|SetCharSide (* (Math|Float|Sign(Float) (.Y (Math|Vector|BreakVector (Math|Vector|UnrotateVector _returnvalue_4 (Transformation|GetWorldRotation (Variables|Default|GetCamera)))))) (- 1.0 (Math|Vector|DotProduct (Class|KismetMathLibrary|VectorNormal2D (Math|Vector|GetForwardVector _camera) 0.0001) (Class|KismetMathLibrary|VectorNormal2D _returnvalue_4 0.0001))))))
  (bind _output_get_2 (Variables|Default|SetReticleSide (* (Math|Float|Sign(Float) (.Y (Math|Vector|BreakVector (Math|Vector|UnrotateVector _returnvalue_7 (Transformation|GetWorldRotation (Variables|Default|GetCamera)))))) (- 1.0 (Math|Vector|DotProduct (Class|KismetMathLibrary|VectorNormal2D (Math|Vector|GetForwardVector _camera_2) 0.0001) (Class|KismetMathLibrary|VectorNormal2D _returnvalue_7 0.0001))))))
  (if (Variables|Default|GetTrackReticle)
    (if (Variables|/Game/StylishCombatKit/Main/BP_BaseCharacter.BP_BaseCharacter_C|GetIsLockedOn (Variables|Default|GetPlayerRef))
      (bind _output_get_3 (Variables|Default|SetCamSide (* (Math|Float|Sign(Float) (Variables|Default|GetCharSide)) -1.0)))
      (Variables|Default|SetTargetCamSide _output_get_3)
      (goto _label Reset)
      (else
        (Variables|Default|SetCamSide (Math|Interpolation|FInterpTo (Variables|Default|GetCamSide) (Variables|Default|GetTargetCamSide) (Utilities|Time|GetWorldDeltaSeconds) 5.0))
        (Variables|Default|SetTargetCamSide (Math|Interpolation|FInterpTo (Variables|Default|GetTargetCamSide) (Math|Float|Sign(Float) (Variables|Default|GetTargetCamSide)) (Utilities|Time|GetWorldDeltaSeconds) 1.0))
        (if (select (== (Math|Float|Sign(Float) (Variables|Default|GetTargetCamSide)) 1.0) (<= (- _output_get_2 _output_get) _returnvalue_6) (>= (- _output_get_2 _output_get) (* _returnvalue_6 -1.0)))
          (if (Math|Float|NearlyEqual(Float) (Variables|Default|GetCamSide) (Variables|Default|GetTargetCamSide) 0.01)
            (Utilities|FlowControl|DoOnce false :!label _label
              (:Completed
                (Variables|Default|SetTargetCamSide (* (Math|Float|Sign(Float) (Variables|Default|GetTargetCamSide)) -0.2))))
            (else
              (goto _label Reset)))
          (else
            (goto _label Reset)))))))

(event Custom|CamReset
  (bind _playerref (Variables|Default|GetPlayerRef))
  (bind _inputvector (Variables|/Game/StylishCombatKit/Main/BP_BaseCharacter.BP_BaseCharacter_C|GetInputVector _playerref))
  (bind (_x _y) (Math|Vector2D|BreakVector2D _inputvector))
  (Variables|Default|SetResetting true)
  (Variables|Default|SetResetRotation (Math|Rotator|MakeRotator 0.0 -5.0 (Math|Float|SelectFloat (.Yaw (Math|Rotator|BreakRotator (Math|Rotator|MakeRotfromX (Math|Vector|RotateVector (Math|Conversions|ToVector(Vector2D) (Math|Vector2D|MakeVector2D _y _x)) (Default|CameraYaw _playerref))))) (.Yaw (Math|Rotator|BreakRotator (Transformation|GetActorRotation (Variables|Default|GetPlayerRef)))) (>= (Math|Vector2D|Vector2DLength _inputvector) (Variables|/Game/StylishCombatKit/Main/BP_BaseCharacter.BP_BaseCharacter_C|GetWalkThreshold _playerref))))))

(event Custom|ControlRotation
  (params (DeltaRotation :type Rotator))
  (bind _returnvalue (Transformation|GetActorRotation))
  (bind _returnvalue_2 (Math|Rotator|CombineRotators DeltaRotation _returnvalue))
  (bind (_roll _pitch _yaw) (Math|Rotator|BreakRotator _returnvalue_2))
  ;[1 1 1] Update camera rotation
  (if (not (Variables|Default|GetResetting))
    (Transformation|SetActorRotation (Math|Rotator|MakeRotator 0.0 (Math|Float|Clamp(Float) _pitch -85.0 85.0) _yaw))))

(event Custom|CamUpdateReticle
  (bind _camera (Variables|Default|GetCamera))
  (bind _playerref (Variables|Default|GetPlayerRef))
  (bind _playerref_2 (Variables|Default|GetPlayerRef))
  (bind _returnvalue (Transformation|GetWorldLocation _camera))
  (bind _returnvalue_2 (Transformation|GetWorldRotation _camera))
  (bind _reticleref (Variables|/Game/StylishCombatKit/Main/BP_BaseCharacter.BP_BaseCharacter_C|GetReticleRef _playerref))
  (bind _reticleref_2 (Variables|/Game/StylishCombatKit/Main/BP_BaseCharacter.BP_BaseCharacter_C|GetReticleRef _playerref_2))
  (bind _returnvalue_3 (Transformation|GetActorLocation _reticleref_2))
  (bind _returnvalue_4 (- _returnvalue_3 _returnvalue))
  (bind _returnvalue_5 (Math|Vector|UnrotateVector _returnvalue_4 _returnvalue_2))
  (bind _returnvalue_6 (Math|Rotator|MakeRotfromX _returnvalue_5))
  (bind (_roll _pitch _yaw) (Math|Rotator|BreakRotator _returnvalue_6))
  (Variables|/Game/Blueprints/BP_Reticle.BP_Reticle_C|SetAngleOffset _reticleref (Math|Rotator|MakeRotator 0.0 _pitch _yaw))
  (Default|UpdateReticle _reticleref))

(event EventBeginPlay
  ;[1 1 1] Initialize
  (bind _asgm_combat_game_mode (Utilities|Casting|CastToGM_CombatGameMode (Game|GetGameMode)))
  (bind _output_get (Variables|Default|SetGameModeRef _asgm_combat_game_mode))
  (bind _output_get_2 (Variables|/Game/StylishCombatKit/Main/GM_CombatGameMode.GM_CombatGameMode_C|SetCameraRef _output_get self))
  (Game|Player|SetViewTargetwithBlend (Game|GetPlayerController 0) _output_get_2 0.0 "VTBlend_Linear" 0.0 false)
  (bind _asbp_base_character (Utilities|Casting|CastToBP_BaseCharacter (Game|GetPlayerCharacter 0)))
  (Variables|Default|SetPlayerRef _asbp_base_character))

(event EventTick
  (params (DeltaSeconds :type Float%20%28single-precision%29))
  (CallFunction|SetLocation)
  (CallFunction|SetRotation)
  (CallFunction|SetZoom)
  (CallFunction|SetFOV)
  (CallFunction|DetectSide))

(fn ConstructionScript)