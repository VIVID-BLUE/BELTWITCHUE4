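; Large air blast projectile for the combat kit, a child projectile that carries a damaging hitbox which launches targets upward.
; On initialize it spawns and activates a sphere BP_Hitbox attached to its capsule and switches movement to flying.
; If the owner is in an aim animation, it pitches toward the lock-on target or otherwise the reticle.
; After a zero-length delay, it sets projectile velocity along its forward vector.
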(event EventInitialize
  ;[1 1 1] Initialize
  (|CallParentFunction)
  (bind _returnvalue (Game|SpawnActorfromClass "/Game/StylishCombatKit/Misc/BP_Hitbox.BP_Hitbox_C" (Transformation|GetActorTransform) "AlwaysSpawn" 0 0))
  (Variables|/Game/StylishCombatKit/Misc/BP_Hitbox.BP_Hitbox_C|SetOwnerCharacter _returnvalue self)
  (Transformation|AttachComponentToComponent _returnvalue (Variables|Default|GetCapsuleComponent) "None" "KeepWorld" "KeepWorld" "KeepWorld" true)
  (Utilities|Array|Add (Variables|Default|GetHitboxes) _returnvalue)
  (Components|Sphere|SetSphereRadius (Variables|/Game/StylishCombatKit/Misc/BP_Hitbox.BP_Hitbox_C|GetHitbox _returnvalue) 4.0 true)
  (Variables|/Game/StylishCombatKit/Misc/BP_Hitbox.BP_Hitbox_C|SetHitData _returnvalue (Utilities|Struct|MakeStruct_HitData 1 "0.000000,0.000000,500.000000" 15.0 1 0.05 0.1 5.0))
  (Default|Activate _returnvalue true)
  (Pawn|Components|CharacterMovement|SetMovementMode (Variables|Character|GetCharacterMovement) "MOVE_Flying" 0)
  (Transformation|AddActorLocalRotation (Math|Rotator|SelectRotator (Math|Rotator|SelectRotator (Math|Rotator|MakeRotator 0.0 (.Pitch (Math|Rotator|BreakRotator (Math|Rotator|FindLookatRotation (Transformation|GetSocketLocation (Variables|/Script/Engine.Character|GetMesh (Variables|Default|GetOwnerCharacter)) "spine_03") (Transformation|GetSocketLocation (Variables|/Script/Engine.Character|GetMesh (Variables|/Game/StylishCombatKit/Main/BP_BaseCharacter.BP_BaseCharacter_C|GetLockOnTarget (Variables|Default|GetOwnerCharacter))) "Target")))) 0.0) (Math|Rotator|MakeRotator 0.0 (.Pitch (Math|Rotator|BreakRotator (Math|Rotator|FindLookatRotation (Transformation|GetSocketLocation (Variables|/Script/Engine.Character|GetMesh (Variables|Default|GetOwnerCharacter)) "spine_03") (Transformation|GetActorLocation (Variables|/Game/StylishCombatKit/Main/BP_BaseCharacter.BP_BaseCharacter_C|GetReticleRef (Variables|Default|GetOwnerCharacter)))))) 0.0) (Variables|/Game/StylishCombatKit/Main/BP_BaseCharacter.BP_BaseCharacter_C|GetIsLockedOn (Variables|Default|GetOwnerCharacter))) "0, 0, 0" (Variables|/Game/StylishCombatKit/Main/BP_BaseCharacter.BP_BaseCharacter_C|GetAimAnim (Variables|Default|GetOwnerCharacter))) false false)
  (Utilities|FlowControl|Delay 0.0)
  (bind _output_get (Variables|Default|SetProjectileVelocity (* (Transformation|GetActorForwardVector) (Variables|Default|GetSpeed))))
  (Variables|Default|SetPreviousFrameVelocity _output_get))

(fn ConstructionScript
  (|CallParentFunction))