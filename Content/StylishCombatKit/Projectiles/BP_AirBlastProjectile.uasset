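; Air blast projectile for the combat kit, a character-based child of a projectile parent that flies at the owner's lock-on or aim target.
; On Initialize it attaches and activates a small spherical BP_Hitbox with light damage, stun and launch data, then switches movement to Flying.
; It rotates once toward the locked target's "Target" socket or the owner's reticle, then after a zero-length delay sets forward velocity from Speed.
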(event EventSpawnTrail
  ;[1 1 1] Initialize
  (|CallParentFunction))

(event EventInitialize
  (bind _returnvalue (Transformation|GetActorLocation))
  ;[1 1 1] Initialize
  (|CallParentFunction)
  (bind _returnvalue_2 (Game|SpawnActorfromClass "/Game/StylishCombatKit/Misc/BP_Hitbox.BP_Hitbox_C" (Transformation|GetActorTransform) "AlwaysSpawn" 0 0))
  (Variables|/Game/StylishCombatKit/Misc/BP_Hitbox.BP_Hitbox_C|SetOwnerCharacter _returnvalue_2 self)
  (Transformation|AttachComponentToComponent _returnvalue_2 (Variables|Default|GetCapsuleComponent) "None" "KeepWorld" "KeepWorld" "KeepWorld" true)
  (Utilities|Array|Add (Variables|Default|GetHitboxes) _returnvalue_2)
  (Components|Sphere|SetSphereRadius (Variables|/Game/StylishCombatKit/Misc/BP_Hitbox.BP_Hitbox_C|GetHitbox _returnvalue_2) 35.0 true)
  (Variables|/Game/StylishCombatKit/Misc/BP_Hitbox.BP_Hitbox_C|SetHitData _returnvalue_2 (Utilities|Struct|MakeStruct_HitData 1 "0.000000,0.000000,300.000000" 1.5 1 0.001 0.1 2.0 0.4 0.4))
  (Default|Activate _returnvalue_2 true)
  (Pawn|Components|CharacterMovement|SetMovementMode (Variables|Character|GetCharacterMovement) "MOVE_Flying" 0)
  (Transformation|SetActorRotation (Math|Rotator|SelectRotator (Math|Rotator|MakeRotator 0.0 (.Pitch (Math|Rotator|BreakRotator (Math|Rotator|FindLookatRotation _returnvalue (Transformation|GetSocketLocation (Variables|/Script/Engine.Character|GetMesh (Variables|/Game/StylishCombatKit/Main/BP_BaseCharacter.BP_BaseCharacter_C|GetLockOnTarget (Variables|Default|GetOwnerCharacter))) "Target")))) (.Yaw (Math|Rotator|BreakRotator (Math|Rotator|FindLookatRotation _returnvalue (Transformation|GetSocketLocation (Variables|/Script/Engine.Character|GetMesh (Variables|/Game/StylishCombatKit/Main/BP_BaseCharacter.BP_BaseCharacter_C|GetLockOnTarget (Variables|Default|GetOwnerCharacter))) "Target"))))) (Math|Rotator|MakeRotator 0.0 (.Pitch (Math|Rotator|BreakRotator (Math|Rotator|FindLookatRotation _returnvalue (Transformation|GetActorLocation (Variables|/Game/StylishCombatKit/Main/BP_BaseCharacter.BP_BaseCharacter_C|GetReticleRef (Variables|Default|GetOwnerCharacter)))))) (.Yaw (Math|Rotator|BreakRotator (Math|Rotator|FindLookatRotation _returnvalue (Transformation|GetActorLocation (Variables|/Game/StylishCombatKit/Main/BP_BaseCharacter.BP_BaseCharacter_C|GetReticleRef (Variables|Default|GetOwnerCharacter))))))) (Variables|/Game/StylishCombatKit/Main/BP_BaseCharacter.BP_BaseCharacter_C|GetIsLockedOn (Variables|Default|GetOwnerCharacter))))
  (Utilities|FlowControl|Delay 0.0)
  (bind _output_get (Variables|Default|SetProjectileVelocity (* (Transformation|GetActorForwardVector) (Variables|Default|GetSpeed))))
  (Variables|Default|SetPreviousFrameVelocity _output_get))

(fn ConstructionScript
  (|CallParentFunction))