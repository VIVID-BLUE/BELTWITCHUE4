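; Shotgun pellet projectile for the combat kit, where a center pellet fans out copies of itself in a random forward cone.
; Each pellet attaches a small hitbox, flies via CharacterMovement, and when aiming pitches toward the lock-on target or reticle.
; Before hit checks, pellets past a distance threshold switch their hitboxes' launch vector and type to a purely upward launch.
; An Instigator-pellet distance check exists but is unconnected.
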(event EventTick
  (params (DeltaSeconds :type Float%20%28single-precision%29))
  (|CallParentFunction DeltaSeconds)
  (CallFunction|PreHitCollision))

(event EventPreHitCollision
  (for _array_element (Variables|Default|GetHitboxes)
    (if (>= (Variables|Default|GetDistanceTraveled) 5e+02)
      (Utilities|Struct|SetmembersinStruct_HitData (Variables|/Game/StylishCombatKit/Misc/BP_Hitbox.BP_Hitbox_C|GetHitData _array_element) "0.000000,0.000000,400.000000" 1))))

(event EventInitialize
  (bind _returnvalue (Transformation|GetActorTransform))
  (bind (_location _rotation _scale) (Math|Transform|BreakTransform _returnvalue))
  ;[1 1 1] Initialize
  (|CallParentFunction)
  (CallFunction|SpawnTrail)
  (if (Variables|Default|GetCenterPellet)
    (for _index (range 0 20)
      (bind _returnvalue_2 (Game|SpawnActorfromClass (Utilities|GetClass self) (Math|Transform|MakeTransform _location (Math|Rotator|MakeRotfromX (Math|Random|RandomUnitVectorinConeinDegrees (Transformation|GetActorForwardVector) 2e+01)) _scale) "AlwaysSpawn" (Variables|Default|GetOwnerCharacter) self))
      (Variables|BP_ShotgunPellet_C|SetCenterPellet _returnvalue_2 false)
      (Pawn|SpawnDefaultController _returnvalue_2)
      (Default|Initialize _returnvalue_2)))
  (bind _returnvalue_3 (Game|SpawnActorfromClass "/Game/StylishCombatKit/Misc/BP_Hitbox.BP_Hitbox_C" (Transformation|GetActorTransform) "AlwaysSpawn" 0 0))
  (Variables|/Game/StylishCombatKit/Misc/BP_Hitbox.BP_Hitbox_C|SetOwnerCharacter _returnvalue_3 self)
  (Transformation|AttachComponentToComponent _returnvalue_3 (Variables|Default|GetCapsuleComponent) "None" "KeepWorld" "KeepWorld" "KeepWorld" true)
  (Utilities|Array|Add (Variables|Default|GetHitboxes) _returnvalue_3)
  (Components|Sphere|SetSphereRadius (Variables|/Game/StylishCombatKit/Misc/BP_Hitbox.BP_Hitbox_C|GetHitbox _returnvalue_3) 5.0 true)
  (Variables|/Game/StylishCombatKit/Misc/BP_Hitbox.BP_Hitbox_C|SetHitData _returnvalue_3 (Utilities|Struct|MakeStruct_HitData 1 "1500.000000,0.000000,750.000000" 5.0 2 0.05 0.1 1.0 0.1 0.1))
  (Default|Activate _returnvalue_3 true)
  (Pawn|Components|CharacterMovement|SetMovementMode (Variables|Character|GetCharacterMovement) "MOVE_Flying" 0)
  (Transformation|AddActorLocalRotation (Math|Rotator|SelectRotator (Math|Rotator|SelectRotator (Math|Rotator|MakeRotator 0.0 (.Pitch (Math|Rotator|BreakRotator (Math|Rotator|FindLookatRotation (Transformation|GetSocketLocation (Variables|/Script/Engine.Character|GetMesh (Variables|Default|GetOwnerCharacter)) "spine_03") (Transformation|GetSocketLocation (Variables|/Script/Engine.Character|GetMesh (Variables|/Game/StylishCombatKit/Main/BP_BaseCharacter.BP_BaseCharacter_C|GetLockOnTarget (Variables|Default|GetOwnerCharacter))) "Target")))) 0.0) (Math|Rotator|MakeRotator 0.0 (.Pitch (Math|Rotator|BreakRotator (Math|Rotator|FindLookatRotation (Transformation|GetSocketLocation (Variables|/Script/Engine.Character|GetMesh (Variables|Default|GetOwnerCharacter)) "spine_03") (Transformation|GetActorLocation (Variables|/Game/StylishCombatKit/Main/BP_BaseCharacter.BP_BaseCharacter_C|GetReticleRef (Variables|Default|GetOwnerCharacter)))))) 0.0) (Variables|/Game/StylishCombatKit/Main/BP_BaseCharacter.BP_BaseCharacter_C|GetIsLockedOn (Variables|Default|GetOwnerCharacter))) "0, 0, 0" (Variables|/Game/StylishCombatKit/Main/BP_BaseCharacter.BP_BaseCharacter_C|GetAimAnim (Variables|Default|GetOwnerCharacter))) false false)
  (Utilities|FlowControl|Delay 0.0)
  (bind _output_get (Variables|Default|SetProjectileVelocity (* (Transformation|GetActorForwardVector) (Variables|Default|GetSpeed))))
  (Variables|Default|SetPreviousFrameVelocity _output_get))

(fn ConstructionScript
  (|CallParentFunction))