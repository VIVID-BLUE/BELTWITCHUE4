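; World-space aiming reticle owned by a BP_BaseCharacter, drawn as a material billboard that resizes on lock-on changes.
; ReticleControl turns pitch/yaw input into a clamped camera-relative angle offset and scaled camera rotation, with edge damping and a focus-aim multiplier.
; UpdateReticle snaps to the lock-on target or line-traces from the character's depth along the aim, setting DetectedTarget and coloring red for hurtboxes, green for weak points.
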(event Custom|UpdateReticle
  (bind _ownerref (Variables|Default|GetOwnerRef))
  (bind _ownerref_2 (Variables|Default|GetOwnerRef))
  (bind _angleoffset (Variables|Default|GetAngleOffset))
  (bind _lockontarget (Variables|/Game/StylishCombatKit/Main/BP_BaseCharacter.BP_BaseCharacter_C|GetLockOnTarget _ownerref))
  (bind _gamemoderef (Variables|/Game/StylishCombatKit/Main/BP_BaseCharacter.BP_BaseCharacter_C|GetGameModeRef _ownerref_2))
  (bind _cameraref (Variables|/Game/StylishCombatKit/Main/GM_CombatGameMode.GM_CombatGameMode_C|GetCameraRef _gamemoderef))
  (bind _camera (Variables|/Game/StylishCombatKit/Main/BP_PlayerCamera.BP_PlayerCamera_C|GetCamera _cameraref))
  (bind _returnvalue (Transformation|GetWorldLocation _camera))
  (bind _returnvalue_2 (Transformation|GetWorldRotation _camera))
  (bind _returnvalue_3 (Math|Rotator|CombineRotators _angleoffset _returnvalue_2))
  (bind _returnvalue_4 (Math|Vector|GetForwardVector _returnvalue_3))
  (bind _returnvalue_5 (* _returnvalue_4 4e+03))
  (bind _returnvalue_6 (+ _returnvalue _returnvalue_5))
  (if (Variables|/Game/StylishCombatKit/Main/BP_BaseCharacter.BP_BaseCharacter_C|GetIsLockedOn _ownerref)
    (Transformation|SetActorLocation (+ (Transformation|GetSocketLocation (Variables|/Script/Engine.Character|GetMesh _lockontarget) "Target") (* _returnvalue_4 -25.0)) false false)
    (Variables|Default|SetDetectedTarget _lockontarget)
    (Rendering|Material|SetVectorParameterValue (Variables|Default|GetReticleMat) "Color" "(R=1.000000,G=0.000000,B=0.000000,A=1.000000)" :!class /Script/Engine.MaterialInstanceDynamic)
    (else
      (bind (_outhit _returnvalue_7) (Collision|LineTraceForObjects (+ (* _returnvalue_4 (Math|Float|SafeDivide (.X (Math|Vector|BreakVector (Math|Vector|UnrotateVector (- (Transformation|GetActorLocation (Variables|Default|GetOwnerRef)) _returnvalue) _returnvalue_2))) (.X (Math|Vector|BreakVector (Math|Vector|UnrotateVector _returnvalue_4 _returnvalue_2))))) _returnvalue) _returnvalue_6 (Utilities|Array|MakeArray "ObjectTypeQuery1" "ObjectTypeQuery8") false (Utilities|Array|MakeArray (Variables|Default|GetOwnerRef)) "None" true "(R=1.000000,G=0.000000,B=0.000000,A=1.000000)" "(R=0.000000,G=1.000000,B=0.000000,A=1.000000)" 1.0))
      (Transformation|SetActorLocation (Math|Vector|SelectVector (.Location (Collision|BreakHitResult _outhit)) _returnvalue_6 _returnvalue_7) false false)
      (bind _asbp_base_character (Utilities|Casting|CastToBP_BaseCharacter (.HitActor (Collision|BreakHitResult _outhit)))
        (:then
          (Variables|Default|SetDetectedTarget _asbp_base_character)
          (bind _ascapsule_collision (Utilities|Casting|CastToCapsuleComponent (.HitComponent (Collision|BreakHitResult _outhit)))
            (:then
              (Rendering|Material|SetVectorParameterValue (Variables|Default|GetReticleMat) "Color" (select (Utilities|Array|ContainsItem (Variables|/Game/StylishCombatKit/Main/BP_BaseCharacter.BP_BaseCharacter_C|GetWeakHurtboxes _asbp_base_character) _ascapsule_collision) "(R=0.000000,G=1.000000,B=0.001896,A=1.000000)" "(R=1.000000,G=0.000000,B=0.000000,A=1.000000)") :!class /Script/Engine.MaterialInstanceDynamic))
            (:CastFailed
              (Rendering|Material|SetVectorParameterValue (Variables|Default|GetReticleMat) "Color" "(R=1.000000,G=1.000000,B=1.000000,A=1.000000)" :!class /Script/Engine.MaterialInstanceDynamic :!label _label))))
        (:CastFailed
          (Variables|Default|SetDetectedTarget 0)
          (goto _label))))))

(event Custom|ReticleControl
  (params (Pitch :type Float%20%28single-precision%29) (Yaw :type Float%20%28single-precision%29))
  (bind _returnvalue (Transformation|GetActorLocation))
  (bind _returnvalue_2 (Transformation|GetActorLocation))
  (bind _aimspeedmultiplier (Variables|Default|GetAimSpeedMultiplier))
  (bind _aimspeedmultiplier_2 (Variables|Default|GetAimSpeedMultiplier))
  (bind _camspeedmultiplier (Variables|Default|GetCamSpeedMultiplier))
  (bind _ownerref (Variables|Default|GetOwnerRef))
  (bind _ownerref_2 (Variables|Default|GetOwnerRef))
  (bind _maxpitch (Variables|Default|GetMaxPitch))
  (bind _ownerref_3 (Variables|Default|GetOwnerRef))
  (bind _ownerref_4 (Variables|Default|GetOwnerRef))
  (bind _maxpitch_2 (Variables|Default|GetMaxPitch))
  (bind _maxyaw (Variables|Default|GetMaxYaw))
  (bind _ownerref_5 (Variables|Default|GetOwnerRef))
  (bind _returnvalue_3 (* _maxyaw 1.1))
  (bind _returnvalue_4 (* _maxpitch_2 1.1))
  (bind _playercontrollerref (Variables|/Game/StylishCombatKit/Main/BP_BaseCharacter.BP_BaseCharacter_C|GetPlayerControllerRef _ownerref_3))
  (bind _focusaim (Variables|/Game/StylishCombatKit/Main/BP_BaseCharacter.BP_BaseCharacter_C|GetFocusAim _ownerref))
  (bind _focusaim_2 (Variables|/Game/StylishCombatKit/Main/BP_BaseCharacter.BP_BaseCharacter_C|GetFocusAim _ownerref_2))
  (bind _gamemoderef (Variables|/Game/StylishCombatKit/Main/BP_BaseCharacter.BP_BaseCharacter_C|GetGameModeRef _ownerref_5))
  (bind _gamemoderef_2 (Variables|/Game/StylishCombatKit/Main/BP_BaseCharacter.BP_BaseCharacter_C|GetGameModeRef _ownerref_4))
  (bind _returnvalue_5 (Math|Float|SelectFloat _aimspeedmultiplier 1.0 _focusaim_2))
  (bind _returnvalue_6 (Math|Float|SelectFloat _aimspeedmultiplier_2 1.0 _focusaim))
  (bind _cameraref (Variables|/Game/StylishCombatKit/Main/GM_CombatGameMode.GM_CombatGameMode_C|GetCameraRef _gamemoderef))
  (bind _cameraref_2 (Variables|/Game/StylishCombatKit/Main/GM_CombatGameMode.GM_CombatGameMode_C|GetCameraRef _gamemoderef_2))
  (bind _camera (Variables|/Game/StylishCombatKit/Main/BP_PlayerCamera.BP_PlayerCamera_C|GetCamera _cameraref))
  (bind _camera_2 (Variables|/Game/StylishCombatKit/Main/BP_PlayerCamera.BP_PlayerCamera_C|GetCamera _cameraref_2))
  (bind _returnvalue_7 (Transformation|GetWorldLocation _camera))
  (bind _returnvalue_8 (Transformation|GetWorldRotation _camera))
  (bind _returnvalue_9 (Transformation|GetWorldLocation _camera_2))
  (bind _returnvalue_10 (Transformation|GetWorldRotation _camera_2))
  (bind _returnvalue_11 (- _returnvalue _returnvalue_7))
  (bind _returnvalue_12 (- _returnvalue_2 _returnvalue_9))
  (bind _returnvalue_13 (Math|Vector|UnrotateVector _returnvalue_11 _returnvalue_8))
  (bind _returnvalue_14 (Math|Vector|UnrotateVector _returnvalue_12 _returnvalue_10))
  (bind _returnvalue_15 (Math|Rotator|MakeRotfromX _returnvalue_13))
  (bind _returnvalue_16 (Math|Rotator|MakeRotfromX _returnvalue_14))
  (bind (_roll _pitch _yaw) (Math|Rotator|BreakRotator _returnvalue_15))
  (bind (_roll_2 _pitch_2 _yaw_2) (Math|Rotator|BreakRotator _returnvalue_16))
  (if (Variables|Default|GetMovingReticle)
    (if (Math|Boolean|ORBoolean (Variables|Default|GetOneFrameOverridePosition) (Variables|/Game/StylishCombatKit/Main/BP_PlayerCamera.BP_PlayerCamera_C|GetResetting _cameraref) (not (Variables|/Game/StylishCombatKit/Main/BP_PlayerCamera.BP_PlayerCamera_C|GetTrackReticle _cameraref)))
      (Variables|Default|SetOneFrameOverridePosition false)
      (else
        (Variables|Default|SetAngleOffset (Math|Rotator|MakeRotator 0.0 _pitch _yaw))))
    (bind _output_get (Variables|Default|SetAngleOffset (select (Variables|/Game/StylishCombatKit/Main/BP_BaseCharacter.BP_BaseCharacter_C|GetIsLockedOn (Variables|Default|GetOwnerRef)) (Math|Rotator|MakeRotator 0.0 _pitch_2 _yaw_2) (Math|Rotator|MakeRotator 0.0 (Math|Float|Clamp(Float) (+ (.Pitch (Math|Rotator|BreakRotator (Variables|Default|GetAngleOffset))) (* Pitch (Variables|Default|GetReticleMoveSpeed) -1.0 (Math|Float|MapRangeClamped (- _returnvalue_4 (Math|Float|Absolute(Float) (.Pitch (Math|Rotator|BreakRotator (Variables|Default|GetAngleOffset))))) 0.0 _returnvalue_4 0.75 1.0) _returnvalue_6)) (* _returnvalue_4 -1.0) _returnvalue_4) (Math|Float|Clamp(Float) (+ (.Yaw (Math|Rotator|BreakRotator (Variables|Default|GetAngleOffset))) (* Yaw (Variables|Default|GetReticleMoveSpeed) (Math|Float|MapRangeClamped (- _returnvalue_3 (Math|Float|Absolute(Float) (.Yaw (Math|Rotator|BreakRotator (Variables|Default|GetAngleOffset))))) 0.0 _returnvalue_3 0.75 1.0) _returnvalue_6)) (* _returnvalue_3 -1.0) _returnvalue_3))))))
  (Default|CameraYaw _playercontrollerref (* Yaw (Math|Float|SelectFloat (+ (* (Math|Float|MapRangeUnclamped (Math|Float|Absolute(Float) (.Yaw (Math|Rotator|BreakRotator _output_get))) 0.0 35.0 0.0 1.0) 0.5) 0.5) 1.0 (Variables|Default|GetMovingReticle)) _camspeedmultiplier _returnvalue_5))
  (Default|CameraPitch _playercontrollerref (* Pitch (Math|Float|SelectFloat (+ (* (Math|Float|SelectFloat 1.0 (Math|Float|MapRangeUnclamped (Math|Float|Absolute(Float) (.Pitch (Math|Rotator|BreakRotator _output_get))) 0.0 2e+01 0.0 1.0) (and (> (Math|Float|Absolute(Float) (.Pitch (Math|Rotator|BreakRotator (Transformation|GetWorldRotation (Variables|/Game/StylishCombatKit/Main/BP_PlayerCamera.BP_PlayerCamera_C|GetCamera (Variables|/Game/StylishCombatKit/Main/GM_CombatGameMode.GM_CombatGameMode_C|GetCameraRef (Variables|/Game/StylishCombatKit/Main/BP_BaseCharacter.BP_BaseCharacter_C|GetGameModeRef (Variables|Default|GetOwnerRef)))))))) _maxpitch) (== _maxpitch (.Pitch (Math|Rotator|BreakRotator (Variables|Default|GetAngleOffset)))))) 0.5) 0.5) 1.0 (Variables|Default|GetMovingReticle)) _camspeedmultiplier _returnvalue_5))
  (CallFunction|UpdateReticle))

(event Custom|LockChange
  (params (Locked :type Boolean))
  (bind _returnvalue (select Locked 5e+01 1e+02))
  (bind _materialbillboard (Variables|Default|GetMaterialBillboard))
  (bind _structout (Utilities|Struct|SetmembersinMaterialSpriteElement (Utilities|Array|Get(acopy) (Variables|/Script/Engine.MaterialBillboardComponent|GetElements _materialbillboard)) _returnvalue _returnvalue))
  (Class|MaterialBillboardComponent|SetElements _materialbillboard (Utilities|Array|MakeArray _structout)))

(event EventBeginPlay
  (bind _materialbillboard (Variables|Default|GetMaterialBillboard))
  (bind _asbp_base_character (Utilities|Casting|CastToBP_BaseCharacter (Components|GetOwner)))
  (Variables|Default|SetOwnerRef _asbp_base_character)
  (bind _returnvalue (Rendering|Material|CreateDynamicMaterialInstance _materialbillboard 0 (Rendering|Material|GetMaterial _materialbillboard 0) "None" :!class /Script/Engine.PrimitiveComponent))
  (Variables|Default|SetReticleMat _returnvalue))

(event Collision|EventActorBeginOverlap
  (params (OtherActor :type Actor%20Object%20Reference)))

(event EventTick
  (params (DeltaSeconds :type Float%20%28single-precision%29))
  (if (Variables|/Game/StylishCombatKit/Main/BP_BaseCharacter.BP_BaseCharacter_C|GetIsLockedOn (Variables|Default|GetOwnerRef))
    (|DoOnceMultiInput :!label _label
      (:A%20Out
        (goto _label_2 Reset%20In))
      (:Reset%20Out
        (|DoOnceMultiInput :!label _label_2
          (:A%20Out
            (CallFunction|LockChange false))
          (:Reset%20Out
            (CallFunction|LockChange true)))))
    (else
      (goto _label Reset%20In))))

(fn ConstructionScript)