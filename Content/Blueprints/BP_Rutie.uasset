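; Rutie is a work-in-progress player character Blueprint with camera-relative movement, jump, dodge-into-sprint and four cyclable combat styles: TriBurst, Blade, Sniper and Caster.
; Dodge launches the character, starts sprinting and re-arms on a timer.
; Mouse2 acts per style, with timeline FOV zoom for aiming and debug prints for launcher and light magic.
; UpdateMovementSpeed derives walk speed from aim and sprint flags, while attack branches remain empty stubs.
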(event Input|ActionEvents|InputActionJump
  (params (Key :type Key%20Structure))
  ;[1 1 1] Basic Movement
  (:Pressed
    (Character|Jump)))

(event Input|ActionEvents|InputActionAttackButton
  (params (Key :type Key%20Structure))
  (bind _currentstyle (Variables|Default|GetCurrentStyle))
  ;[1 1 1] AttackingWIP
  (:Pressed
    (if (Variables|Default|GetSprint)
      (switch int _currentstyle
        (:0
          _)
        (:1
          _)
        (:2
          _)
        (:3
          _))
      (CallFunction|StopSprint)
      (else
        (switch int _currentstyle))))
  (:Released
    (switch int _currentstyle)))

(event Input|ActionEvents|InputActionMouse2Button
  (params (Key :type Key%20Structure))
  (bind _currentstyle (Variables|Default|GetCurrentStyle))
  (bind _camera1 (Variables|Default|GetCamera1))
  ;[1 1 1] Mouse2FunctionsWIP
  (:Pressed
    (switch int _currentstyle
      (:0
        (Variables|Default|SetTriBurstAim true)
        (Development|PrintString "TriAiming")
        (CallFunction|UpdateMovementSpeed)
        (bind _fov_1 (Timeline|AimTimeline1 Play)
          (:Update
            (Camera|SetFieldOfView _camera1 _fov_1)
            (CallFunction|StopSprint))))
      (:1
        (Development|PrintString "Launcher"))
      (:2
        (Variables|Default|SetSnipeModeAim true)
        (Development|PrintString "SnipeAim")
        (CallFunction|UpdateMovementSpeed)
        (bind _fov_2 (Timeline|AimTimeline2 Play)
          (:Update
            (Camera|SetFieldOfView _camera1 _fov_2)
            (CallFunction|StopSprint))))
      (:3
        (Variables|Default|SetCasterLightCharge true)
        (Development|PrintString "Charging Light Magic!"))))
  (:Released
    (switch int _currentstyle
      (:0
        (Variables|Default|SetTriBurstAim false)
        (Development|PrintString "AimOut")
        (CallFunction|UpdateMovementSpeed)
        (Timeline|AimTimeline1 Reverse))
      (:2
        (Variables|Default|SetSnipeModeAim false)
        (Development|PrintString "Not The Target...")
        (CallFunction|UpdateMovementSpeed)
        (Timeline|AimTimeline2 Reverse))
      (:3
        (Variables|Default|SetCasterLightCharge false)
        (Development|PrintString "Firing Light Magic!")))))

(event Input|ActionEvents|InputActionDodgeButton
  (params (Key :type Key%20Structure))
  (bind _returnvalue (Pawn|GetControlRotation :!class /Script/Engine.Pawn))
  (bind _yaw (Math|Rotator|BreakRotator _returnvalue))
  (bind _returnvalue_2 (Math|Rotator|MakeRotator 0.0 0.0 _yaw))
  ;[1 1 1] Dodge/Sprint WIP
  (:Pressed
    (if (Variables|Default|GetDodge)
      (Variables|Default|SetSprint true)
      (CallFunction|UpdateMovementSpeed)
      (Character|LaunchCharacter (+ (Transformation|GetVelocity) (+ (* (Math|Vector|GetForwardVector _returnvalue_2) (* (stale Input|AxisEvents|InputAxisMoveForward AxisValue) 2.5e+03)) (* (Math|Vector|GetRightVector _returnvalue_2) (* (stale Input|AxisEvents|InputAxisMoveRight AxisValue) 2.5e+03)))) true true)
      (Variables|Default|SetDodge false)
      (Utilities|Time|SetTimerbyFunctionName 0 "SetDodge" 0.5))))

(event Input|AxisEvents|InputAxisMoveRight
  (params (AxisValue :type Float%20%28single-precision%29))
  ;[1 1 1] Basic Movement
  (Pawn|Input|AddMovementInput (Math|Vector|GetRightVector (Math|Rotator|MakeRotator 0.0 0.0 (.Yaw (Math|Rotator|BreakRotator (Pawn|GetControlRotation :!class /Script/Engine.Pawn))))) AxisValue false))

(event Input|AxisEvents|InputAxisMoveForward
  (params (AxisValue :type Float%20%28single-precision%29))
  ;[1 1 1] Basic Movement
  (Pawn|Input|AddMovementInput (Math|Vector|GetForwardVector (Math|Rotator|MakeRotator 0.0 0.0 (.Yaw (Math|Rotator|BreakRotator (Pawn|GetControlRotation :!class /Script/Engine.Pawn))))) AxisValue false))

(event Input|AxisEvents|InputAxisLookPitch
  (params (AxisValue :type Float%20%28single-precision%29))
  ;[1 1 1] Look
  (Pawn|Input|AddControllerPitchInput AxisValue))

(event Input|AxisEvents|InputAxisLookYaw
  (params (AxisValue :type Float%20%28single-precision%29))
  ;[1 1 1] Look
  (Pawn|Input|AddControllerYawInput AxisValue))

(event Input|KeyboardEvents|E
  (params (Key :type Key%20Structure))
  ;[1 1 1] Cycle Styles WIP
  (:Pressed
    (if (>= (Variables|Default|GetCurrentStyle) 3)
      (Variables|Default|SetCurrentStyle 0)
      (else
        (Variables|Default|SetCurrentStyle (+ (Variables|Default|GetCurrentStyle) 1))))
    (CallFunction|SwitchStyle)))

(event Input|KeyboardEvents|Q
  (params (Key :type Key%20Structure))
  ;[1 1 1] Cycle Styles WIP
  (:Pressed
    (if (<= (Variables|Default|GetCurrentStyle) 0)
      (Variables|Default|SetCurrentStyle 3)
      (else
        (Variables|Default|SetCurrentStyle (- (Variables|Default|GetCurrentStyle) 1))))
    (CallFunction|SwitchStyle)))

(event Input|MouseEvents|MouseWheelDown
  (params (Key :type Key%20Structure))
  ;[1 1 1] Cycle Styles WIP
  (:Pressed
    (if (>= (Variables|Default|GetCurrentStyle) 3)
      (Variables|Default|SetCurrentStyle 0)
      (else
        (Variables|Default|SetCurrentStyle (+ (Variables|Default|GetCurrentStyle) 1))))
    (CallFunction|SwitchStyle)))

(event Input|MouseEvents|MouseWheelUp
  (params (Key :type Key%20Structure))
  ;[1 1 1] Cycle Styles WIP
  (:Pressed
    (if (<= (Variables|Default|GetCurrentStyle) 0)
      (Variables|Default|SetCurrentStyle 3)
      (else
        (Variables|Default|SetCurrentStyle (- (Variables|Default|GetCurrentStyle) 1))))
    (CallFunction|SwitchStyle)))

(fn ConstructionScript)

(fn StartSprint
  (Components|Activation|Activate (Variables|Default|GetSprintDust) false)
  (Variables|/Script/Engine.CharacterMovementComponent|SetMaxWalkSpeed (Variables|Character|GetCharacterMovement) (Variables|Default|GetDodgeSpeed)))

(fn StopSprint
  (Components|Activation|Deactivate (Variables|Default|GetSprintDust))
  (Variables|Default|SetSprint false)
  (Variables|/Script/Engine.CharacterMovementComponent|SetMaxWalkSpeed (Variables|Character|GetCharacterMovement) (Variables|Default|GetWalkSpeed)))

(fn SwitchStyle
  (switch int (Variables|Default|GetCurrentStyle)
    (:0
      (Variables|Default|SetTriBurstMode true)
      (Development|PrintString "TriBurst!"))
    (:1
      (Variables|Default|SetBladeMode true)
      (Development|PrintString "Blade!"))
    (:2
      (Variables|Default|SetSnipeMode true)
      (Development|PrintString "Sniper!"))
    (:3
      (Variables|Default|SetCasterMode true)
      (Development|PrintString "Caster!"))))

(fn Sprinting
  (Components|Activation|Deactivate (Variables|Default|GetSprintDust))
  (Variables|Default|SetSprint true)
  (Variables|/Script/Engine.CharacterMovementComponent|SetMaxWalkSpeed (Variables|Character|GetCharacterMovement) (Variables|Default|GetSprintSpeed)))

(fn UpdateMovementSpeed
  (bind _charactermovement (Variables|Character|GetCharacterMovement))
  (bind _sprintdust (Variables|Default|GetSprintDust))
  (if (Variables|Default|GetSnipeModeAim)
    (Variables|/Script/Engine.CharacterMovementComponent|SetMaxWalkSpeed _charactermovement 2.5e+02)
    (elif (Variables|Default|GetTriBurstAim)
      (Variables|/Script/Engine.CharacterMovementComponent|SetMaxWalkSpeed _charactermovement 4e+02)
      (elif (Variables|Default|GetSprint)
        (Components|Activation|Activate _sprintdust false)
        (Variables|/Script/Engine.CharacterMovementComponent|SetMaxWalkSpeed _charactermovement (Variables|Default|GetSprintSpeed))
        (else
          (Components|Activation|Deactivate _sprintdust)
          (Variables|/Script/Engine.CharacterMovementComponent|SetMaxWalkSpeed _charactermovement (Variables|Default|GetWalkSpeed)))))))

(fn SetDodge
  (Variables|Default|SetDodge true))